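; BP_InvenItem is a base inventory item that pairs a data table RowName with a current Amount.
; Getters look up the DTItems row for item info, stackability and max stack size, and derive remaining stack room from Amount.
; A missing row prints an error, with false or -1 returned by the stack queries.
; OnUse and OnDrop are empty, and Amount has a simple getter and setter.
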(fn GetInventoryItemInfo
  (bind _rowname (Variables|Default|GetRowName))
  (bind _returnvalue (Utilities|GetDataTableRow "/Game/Blueprints/Structure/DataTables/DTItems.DTItems" _rowname)
    (:then
      (return _returnvalue))
    (:RowNotFound
      (Development|PrintString 0 (Utilities|String|Append "Row " (Utilities|String|ToString(Name) _rowname) " Not Found!"))
      (return ""))))

(fn GetItemInfo
  (bind _rowname (Variables|Default|GetRowName))
  (bind _returnvalue (Utilities|GetDataTableRow "/Game/Blueprints/Structure/DataTables/DTItems.DTItems" _rowname)
    (:then
      (return (.iteminfo _returnvalue)))
    (:RowNotFound
      (Development|PrintString 0 (Utilities|String|Append "Row " (Utilities|String|ToString(Name) _rowname) " Not Found"))
      (return ""))))

(fn CanStack?
  (bind _rowname (Variables|Default|GetRowName))
  (bind _returnvalue (Utilities|GetDataTableRow "/Game/Blueprints/Structure/DataTables/DTItems.DTItems" _rowname)
    (:then
      (return (.canstack? _returnvalue)))
    (:RowNotFound
      (Development|PrintString 0 (Utilities|String|Append "Row " (Utilities|String|ToString(Name) _rowname) " Not Found"))
      (return false))))

(fn GetMaxStackAmount
  (bind _rowname (Variables|Default|GetRowName))
  (bind _returnvalue (Utilities|GetDataTableRow "/Game/Blueprints/Structure/DataTables/DTItems.DTItems" _rowname)
    (:then
      (return (.maxstackamount _returnvalue)))
    (:RowNotFound
      (Development|PrintString 0 (Utilities|String|Append "Row " (Utilities|String|ToString(Name) _rowname) " Not Found"))
      (return -1))))

(fn GetRoomonStack
  (bind _rowname (Variables|Default|GetRowName))
  (bind _returnvalue (Utilities|GetDataTableRow "/Game/Blueprints/Structure/DataTables/DTItems.DTItems" _rowname)
    (:then
      (return (- (.maxstackamount _returnvalue) (Variables|Default|GetAmount))))
    (:RowNotFound
      (Development|PrintString 0 (Utilities|String|Append "Row " (Utilities|String|ToString(Name) _rowname) " Not Found"))
      (return -1))))

(fn OnUse)

(fn OnDrop)

(fn GetAmount
  (return (Variables|Default|GetAmount)))

(fn SetAmount
  (params (Amount :type Integer))
  (Variables|Default|SetAmount Amount))