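; Base inventory item for equipable gear that grants a stat bonus to a character.
; OnEquip passes the item to the character's equipment component, applies the bonus, and adds the class of EquipItem's returned item to inventory.
; OnUnEquip adds the item to inventory and, only on success, unequips it.
; GiveBonus and RemoveBonus switch on StatType to adjust the stat by BonusAmount; RemoveBonus is not called here.
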(fn OnEquip
  (params (CharacterRef :type BP%20Surviving%20Life%20Character%20Object%20Reference))
  (bind _itemequiped (Default|EquipItem (Variables|/Game/Blueprints/Character/BPSurvivingLifeCharacter.BPSurvivingLifeCharacter_C|GetBP_Equipment CharacterRef) self))
  (CallFunction|GiveBonus CharacterRef)
  (Default|AddItem (Variables|/Game/Blueprints/Character/BPSurvivingLifeCharacter.BPSurvivingLifeCharacter_C|GetBP_Inventory CharacterRef) (Utilities|GetClass _itemequiped) 1))

(fn GiveBonus
  (params (CharacterRef :type BP%20Surviving%20Life%20Character%20Object%20Reference))
  (switch Utilities|FlowControl|Switch|SwitchonEStatType (Variables|Default|GetStatType)
    (:NewEnumerator0
      (Default|GiveStr CharacterRef (Variables|Default|GetBonusAmount)))
    (:NewEnumerator1
      (Default|GiveInt CharacterRef (Variables|Default|GetBonusAmount)))
    (:NewEnumerator2
      (Default|GiveDex CharacterRef (Variables|Default|GetBonusAmount)))
    (:NewEnumerator3
      (Default|GiveConst CharacterRef (Variables|Default|GetBonusAmount)))
    (:NewEnumerator4
      (Default|GiveChr CharacterRef (Variables|Default|GetBonusAmount)))))

(fn OnUnEquip
  (params (CharacterRef :type BP%20Surviving%20Life%20Character%20Object%20Reference))
  (bind _additem_ (Default|AddItem (Variables|/Game/Blueprints/Character/BPSurvivingLifeCharacter.BPSurvivingLifeCharacter_C|GetBP_Inventory CharacterRef) (Utilities|GetClass self) 1))
  (if _additem_
    (Default|UnEquipItem (Variables|/Game/Blueprints/Character/BPSurvivingLifeCharacter.BPSurvivingLifeCharacter_C|GetBP_Equipment CharacterRef) self)))

(fn RemoveBonus
  (params (CharacterRef :type BP%20Surviving%20Life%20Character%20Object%20Reference))
  (switch Utilities|FlowControl|Switch|SwitchonEStatType (Variables|Default|GetStatType)
    (:NewEnumerator0
      (Default|RemoveStr CharacterRef (Variables|Default|GetBonusAmount)))
    (:NewEnumerator1
      (Default|RemoveInt CharacterRef (Variables|Default|GetBonusAmount)))
    (:NewEnumerator2
      (Default|RemoveDex CharacterRef (Variables|Default|GetBonusAmount)))
    (:NewEnumerator3
      (Default|RemoveConst CharacterRef (Variables|Default|GetBonusAmount)))
    (:NewEnumerator4
      (Default|RemoveChr CharacterRef (Variables|Default|GetBonusAmount)))))