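; WeatherModifier is a placeable box volume that changes the temperature felt by BPSurvivingLifeCharacter actors inside it.
; On begin overlap it calls ApplyTemperatureModifier with an optional world-temperature override and an additive area offset.
; On end overlap it clears the override and passes the negated offset to undo the change.
; The construction script sizes the Volume box from the BoxArea variable.
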(event OnComponentBeginOverlap(Volume)
  (params (OverlappedComponent :type Primitive%20Component%20Object%20Reference) (OtherActor :type Actor%20Object%20Reference) (OtherComp :type Primitive%20Component%20Object%20Reference) (OtherBodyIndex :type Integer) (bFromSweep :type Boolean) (SweepResult :type Hit%20Result%20Structure%20%28by%20ref%29))
  (bind _asbpsurviving_life_character (Utilities|Casting|CastToBPSurvivingLifeCharacter OtherActor))
  (Default|ApplyTemperatureModifier _asbpsurviving_life_character (Variables|Default|GetOverrrideLocalWolrdTemp?) (Variables|Default|GetOverritenWorldTemp) (Variables|Default|GetAreaTempModifier)))

(event OnComponentEndOverlap(Volume)
  (params (OverlappedComponent :type Primitive%20Component%20Object%20Reference) (OtherActor :type Actor%20Object%20Reference) (OtherComp :type Primitive%20Component%20Object%20Reference) (OtherBodyIndex :type Integer))
  (bind _asbpsurviving_life_character (Utilities|Casting|CastToBPSurvivingLifeCharacter OtherActor))
  (Default|ApplyTemperatureModifier _asbpsurviving_life_character false 0.0 (* (Variables|Default|GetAreaTempModifier) -1.0)))

(fn ConstructionScript
  (Components|Box|SetBoxExtent (Variables|Default|GetVolume) (Variables|Default|GetBoxArea) true))