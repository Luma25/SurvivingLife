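; Player character for a survival game, handling movement, sprint, crouch, stats and survival needs.
; Looping timers by function name drive stamina, hunger, thirst and body temperature, with empty hunger or thirst draining health.
; Body temperature follows a curve over weather, clothing and area modifiers.
; Interface calls handle pickup, damage and harvesting, while inventory and equipment components feed the HUD-side ICE menu; most stat modifiers are empty stubs.
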(event Custom|DecreaseStamina
  ;[1 1 1] Stamina Compsumtion Helper Function
  ;;[1 1 1] Decrease Stamina
  (if (<= (Math|Float|Clamp(Float) (- (Variables|Attributes|Stamina|GetCurrentStamina) (Variables|Attributes|Stamina|GetStaminaDecreaseAmount)) 0.0 (Variables|Attributes|Stamina|GetMaxStamina)) 0.0)
    (Variables|Attributes|Stamina|SetCurrentStamina 0.0)
    (Attributes|Stamina|ClearStaminaDecreaseTimer)
    (Attributes|Movement|SetSpeedtoWalk)
    (Variables|Attributes|Movement|SetOutOfBreath? true)
    (Utilities|FlowControl|Delay (Variables|Attributes|Movement|GetOutOfBreathDelay))
    (Attributes|Stamina|SetStaminaIncreaseTimer)
    (else
      (Variables|Attributes|Stamina|SetCurrentStamina (Math|Float|Clamp(Float) (- (Variables|Attributes|Stamina|GetCurrentStamina) (Variables|Attributes|Stamina|GetStaminaDecreaseAmount)) 0.0 (Variables|Attributes|Stamina|GetMaxStamina))))))

(event Custom|IncreaseStamina
  (bind _maxstamina (Variables|Attributes|Stamina|GetMaxStamina))
  ;[1 1 1] Stamina Compsumtion Helper Function
  ;;[1 1 1] Increase Stamina
  (if (>= (Math|Float|Clamp(Float) (+ (Variables|Attributes|Stamina|GetCurrentStamina) (Variables|Attributes|Stamina|GetStaminaIncreaseAmount)) 0.0 _maxstamina) _maxstamina)
    (Variables|Attributes|Stamina|SetCurrentStamina (Variables|Attributes|Stamina|GetMaxStamina))
    (Attributes|Stamina|ClearStaminaIncreaseTimer)
    (Variables|Attributes|Movement|SetOutOfBreath? false)
    (else
      (Variables|Attributes|Stamina|SetCurrentStamina (Math|Float|Clamp(Float) (+ (Variables|Attributes|Stamina|GetCurrentStamina) (Variables|Attributes|Stamina|GetStaminaIncreaseAmount)) 0.0 _maxstamina)))))

(event Custom|Use/Equip
  (params (Item :type BP%20Inventory%20Item%20Object%20Reference))
  (bind _self self)
  (bind _icelayoutref (Variables|References|UI|GetIceLayoutRef))
  ;[1 1 1] Use Item
  (Actions|UseItem Item)
  (Default|Reconstruct (Variables|/Game/UI/UI_ICEPanelLayout.UI_ICEPanelLayout_C|GetUI_InventoryPanel _icelayoutref) _self)
  (Default|Reconstruct (Variables|/Game/UI/UI_ICEPanelLayout.UI_ICEPanelLayout_C|GetUI_EquipmentPanel _icelayoutref) _self))

(event EventBeginPlay
  ;[1 1 1] Initial Character Setup
  (Utilities|FlowControl|Sequence
    (:then_0
      (Attributes|RandomizeHungerThirst)
      (Variables|Attributes|SetStats (Utilities|Struct|MakeS_Stats 10 10 10 10 10)))
    (:then_1
      ;;[1 1 1] Create Game HUD
      (bind _returnvalue (UserInterface|CreateWidget "/Game/UI/UI_GameHUD.UI_GameHUD_C" 0 self))
      (bind _output_get (Variables|References|UI|SetGameHUDRef _returnvalue))
      (UserInterface|Viewport|AddtoViewport _output_get 0)
      (References|SetIceLayoutRef))
    (:then_2
      (References|SetWeatherManager)
      (Attributes|Temperature|SetBodyTempTimer))
    (:then_3
      ;;[1 1 1] Deplete Status by time
      (Attributes|Hunger|SetHungerTimer)
      (Attributes|Thirst|SetThirstTimer))))

(event EventMakeDamage
  (params (CharacterRef :type BP%20Surviving%20Life%20Character%20Object%20Reference))
  (Attributes|Health|TakeDamage self (Math|Conversions|ToFloat(Integer) (Stats|Str|GetStr CharacterRef))))

(event Input|ActionEvents|InputActionCrouch
  (params (Key :type Key%20Structure))
  ;[1 1 1] Crouch
  (:Pressed
    (Utilities|FlowControl|FlipFlop
      (:A
        (Attributes|Movement|SetSpeedtoCrouch))
      (:B
        (Attributes|Movement|SetSpeedtoWalk)))))

(event Input|ActionEvents|InputActionInteract
  (params (Key :type Key%20Structure))
  (bind _returnvalue (Transformation|GetActorLocation))
  (bind (_returnvalue_2 _returnvalue2) (|GetPositionforTrace _returnvalue))
  ;[1 1 1] Interact with Item
  (:Pressed
    (bind (_outhit _returnvalue_3) (Collision|SphereTraceForObjects _returnvalue_2 _returnvalue2 (Variables|Actions|GetActionRadius) (Utilities|Array|MakeArray "ObjectTypeQuery2") false 0 "ForDuration" true "(R=1.000000,G=0.000000,B=0.000000,A=1.000000)" "(R=0.000000,G=1.000000,B=0.000000,A=1.000000)" 1.0))
    (if _returnvalue_3
      (if (Utilities|DoesObjectImplementInterface (.HitActor (Collision|BreakHitResult _outhit)) "/Game/Blueprints/Interfaces/BPI_ICE.BPI_ICE_C")
        (Class|BPIICE|PickUp(Message) (.HitActor (Collision|BreakHitResult _outhit)) self)
        (Default|Reconstruct (Variables|/Game/UI/UI_ICEPanelLayout.UI_ICEPanelLayout_C|GetUI_InventoryPanel (Variables|References|UI|GetIceLayoutRef)) self)))))

(event Input|ActionEvents|InputActionSprint
  (params (Key :type Key%20Structure))
  ;[1 1 1] Sprint
  (:Pressed
    (if (Attributes|Stamina|CanSprint?)
      (Attributes|Movement|SetSpeedtoSprint)
      (Attributes|Stamina|SetStaminaDecreaseTimer)
      (Attributes|Stamina|ClearStaminaIncreaseTimer)
      (Variables|Actions|SetIsSprinting? true)))
  (:Released
    (Variables|Actions|SetIsSprinting? false)
    (if (not (Variables|Attributes|Movement|GetOutOfBreath?))
      (Attributes|Movement|SetSpeedtoWalk)
      (if (not (Actions|IsPerformingAction?))
        (Attributes|Stamina|SetStaminaIncreaseTimer)
        (Attributes|Stamina|ClearStaminaDecreaseTimer)))))

(event Input|ActionEvents|InputActionICE_Menu
  (params (Key :type Key%20Structure))
  (bind _returnvalue (Game|GetPlayerController 0))
  ;[1 1 1] Show ICE
  (:Pressed
    (if (Widget|IsVisible (Variables|References|UI|GetIceLayoutRef))
      (Variables|Actions|SetIsInMenu? false)
      (Widget|SetVisibility (Variables|References|UI|GetIceLayoutRef) "Hidden")
      (Input|SetInputModeGameOnly _returnvalue)
      (Variables|/Script/Engine.PlayerController|SetbShowMouseCursor (Game|GetPlayerController 0) false)
      (else
        (Variables|Actions|SetIsInMenu? true)
        (Widget|SetVisibility (Variables|References|UI|GetIceLayoutRef) "Visible")
        (Input|SetInputModeGameandUI _returnvalue (Variables|References|UI|GetIceLayoutRef) "LockAlways" false)
        (Variables|/Script/Engine.PlayerController|SetbShowMouseCursor (Game|GetPlayerController 0) true)))))

(event Input|ActionEvents|InputActionDo
  (params (Key :type Key%20Structure))
  (:Pressed
    (bind _output (|GetOverlappingActor))
    (if (Utilities|DoesObjectImplementInterface _output "/Game/Blueprints/Interfaces/BPI_Damage.BPI_Damage_C")
      (Class|BPIDamage|MakeDamage(Message) _output self)
      (Default|BoxerUp (Variables|Default|GetBP_TraitsSkills) self)
      (elif (Utilities|DoesObjectImplementInterface _output "/Game/Blueprints/Interfaces/BPI_Harvest.BPI_Harvest_C")
        (Class|BPIHarvest|DoOnce(Message) _output 1 self)))))

(event Input|AxisEvents|InputAxisMoveForward
  (params (AxisValue :type Float%20%28single-precision%29))
  ;[1 1 1] Movement
  (if (not (Actions|IsPerformingAction?))
    (Pawn|Input|AddMovementInput (Math|Vector|GetForwardVector (Math|Rotator|MakeRotator 0.0 0.0 (.Yaw (Math|Rotator|BreakRotator (Pawn|GetControlRotation :!class /Script/Engine.Pawn))))) AxisValue false)))

(event Input|AxisEvents|InputAxisMoveSideWays
  (params (AxisValue :type Float%20%28single-precision%29))
  ;[1 1 1] Movement
  (if (not (Actions|IsPerformingAction?))
    (Pawn|Input|AddMovementInput (Math|Vector|GetRightVector (Math|Rotator|MakeRotator 0.0 0.0 (.Yaw (Math|Rotator|BreakRotator (Pawn|GetControlRotation :!class /Script/Engine.Pawn))))) AxisValue false)))

(event Input|KeyboardEvents|1
  (params (Key :type Key%20Structure))
  ;[1 1 1] InventoryDebug
  (:Pressed
    (for _array_element (Default|GetInventory (Variables|Default|GetBP_Inventory))
      (Development|PrintString (Utilities|String|ToString(Name) (Variables|/Game/Blueprints/Inventory/BaseClasses/BP_InventoryItem.BP_InventoryItem_C|GetRowName _array_element))))))

(event Input|KeyboardEvents|3
  (params (Key :type Key%20Structure))
  (bind _stats (Variables|Attributes|GetStats))
  (:Pressed
    (for _array_element (Utilities|Array|MakeArray (.strenght _stats) (.inteligence _stats) (.dextery _stats) (.constitution _stats) (.charisma _stats))
      (Development|PrintString (Utilities|String|ToString(Integer) _array_element)))))

(event Input|KeyboardEvents|2
  (params (Key :type Key%20Structure))
  ;[1 1 1] Equipment Debug
  (:Pressed
    (for _array_element (Default|GetEquipment (Variables|Default|GetBP_Equipment))
      (Development|PrintString (Utilities|String|ToString(Name) (Variables|/Game/Blueprints/Inventory/BaseClasses/BP_InventoryItem.BP_InventoryItem_C|GetRowName _array_element))))))

(fn ConstructionScript
  (Attributes|Movement|SetSpeedtoWalk))

(fn RandomizeHungerThirst
  (Variables|Attributes|Hunger|SetCurrentHunger (Math|Random|RandomFloatinRange 7e+01 9e+01))
  (Variables|Attributes|Thirst|SetCurrentThirst (Math|Random|RandomFloatinRange 7e+01 9e+01)))

(fn DepleteHunger
  (if (<= (Math|Float|Clamp(Float) (- (Variables|Attributes|Hunger|GetCurrentHunger) (Variables|Attributes|Hunger|GetHungerDepletionAmount)) 0.0 (Variables|Attributes|Hunger|GetMaxHunger)) 0.0)
    (Variables|Attributes|Hunger|SetCurrentHunger 0.0)
    (Utilities|Time|ClearTimerbyFunctionName self (Variables|Attributes|Hunger|GetDepleteHungerByTime))
    ;[1 1 1] Lose Health
    (Development|PrintString "Hello")
    (if (Attributes|Health|IsHealthTimerActive)
      (Variables|Attributes|Health|SetHealthDepletionAmount (* (Variables|Attributes|Hunger|GetHungerDepletionAmount) 2.0))
      (else
        (Attributes|Health|SetHealthTimer)))
    (else
      (Variables|Attributes|Hunger|SetCurrentHunger (Math|Float|Clamp(Float) (- (Variables|Attributes|Hunger|GetCurrentHunger) (Variables|Attributes|Hunger|GetHungerDepletionAmount)) 0.0 (Variables|Attributes|Hunger|GetMaxHunger))))))

(fn DepleteThirst
  (if (<= (Math|Float|Clamp(Float) (- (Variables|Attributes|Thirst|GetCurrentThirst) (Variables|Attributes|Thirst|GetThirstDepletionAmount)) 0.0 (Variables|Attributes|Thirst|GetMaxThirst)) 0.0)
    (Variables|Attributes|Thirst|SetCurrentThirst 0.0)
    (Utilities|Time|ClearTimerbyFunctionName self (Variables|Attributes|Thirst|GetDepleteThirstByTime))
    ;[1 1 1] Lose Health
    (Development|PrintString "Dehydration")
    (if (Attributes|Health|IsHealthTimerActive)
      (Variables|Attributes|Health|SetHealthDepletionAmount (* (Variables|Attributes|Thirst|GetThirstDepletionAmount) 2.0))
      (else
        (Attributes|Health|SetHealthTimer)))
    (else
      (Variables|Attributes|Thirst|SetCurrentThirst (Math|Float|Clamp(Float) (- (Variables|Attributes|Thirst|GetCurrentThirst) (Variables|Attributes|Thirst|GetThirstDepletionAmount)) 0.0 (Variables|Attributes|Thirst|GetMaxThirst))))))

(fn DepleteHealth
  (if (<= (Math|Float|Clamp(Float) (- (Variables|Attributes|Health|GetCurrentHealth) (Variables|Attributes|Health|GetHealthDepletionAmount)) 0.0 (Variables|Attributes|Health|GetMaxHealth)) 0.0)
    (Variables|Attributes|Health|SetCurrentHealth 0.0)
    (Utilities|Time|ClearTimerbyFunctionName self (Variables|Attributes|Health|GetDepleteHealthByTime))
    ;[1 1 1] Lose Health
    (Development|PrintString "You are dead")
    (else
      (Variables|Attributes|Health|SetCurrentHealth (Math|Float|Clamp(Float) (- (Variables|Attributes|Health|GetCurrentHealth) (Variables|Attributes|Health|GetHealthDepletionAmount)) 0.0 (Variables|Attributes|Health|GetMaxHealth))))))

(fn AddHunger
  (params (Amount :type Float%20%28single-precision%29))
  (Variables|Attributes|Hunger|SetCurrentHunger (Math|Float|Clamp(Float) (+ Amount (Variables|Attributes|Hunger|GetCurrentHunger)) 0.0 (Variables|Attributes|Hunger|GetMaxHunger)))
  (if (not (Attributes|Hunger|IsHungerTimerActive))
    (Attributes|Hunger|SetHungerTimer)
    (if (and (Attributes|Health|IsHealthTimerActive) (not (Attributes|Thirst|IsThirstTimerActive)))
      (Variables|Attributes|Health|SetHealthDepletionAmount (/ (Variables|Attributes|Health|GetHealthDepletionRate) 2.0))
      (else
        (Utilities|Time|ClearTimerbyFunctionName self (Variables|Attributes|Health|GetDepleteHealthByTime))))))

(fn AddThirst
  (params (Amount :type Float%20%28single-precision%29))
  (Variables|Attributes|Thirst|SetCurrentThirst (Math|Float|Clamp(Float) (+ Amount (Variables|Attributes|Thirst|GetCurrentThirst)) 0.0 (Variables|Attributes|Thirst|GetMaxThirst)))
  (if (not (Attributes|Thirst|IsThirstTimerActive))
    (Attributes|Thirst|SetThirstTimer)
    (if (and (Attributes|Health|IsHealthTimerActive) (not (Attributes|Hunger|IsHungerTimerActive)))
      (Variables|Attributes|Health|SetHealthDepletionAmount (/ (Variables|Attributes|Health|GetHealthDepletionRate) 2.0))
      (else
        (Utilities|Time|ClearTimerbyFunctionName self (Variables|Attributes|Health|GetDepleteHealthByTime))))))

(fn AddHealth
  (params (HealthToAdd :type Float%20%28single-precision%29))
  (Variables|Attributes|Health|SetCurrentHealth (Math|Float|Clamp(Float) (+ HealthToAdd (Variables|Attributes|Health|GetCurrentHealth)) 0.0 (Variables|Attributes|Health|GetMaxHealth))))

(fn IsHealthTimerActive
  (return (Class|KismetSystemLibrary|IsTimerActive self (Variables|Attributes|Health|GetDepleteHealthByTime))))

(fn IsThirstTimerActive
  (return (Class|KismetSystemLibrary|IsTimerActive self (Variables|Attributes|Thirst|GetDepleteThirstByTime))))

(fn IsHungerTimerActive
  (return (Class|KismetSystemLibrary|IsTimerActive self (Variables|Attributes|Hunger|GetDepleteHungerByTime))))

(fn SetThirstTimer
  (Utilities|Time|SetTimerbyFunctionName self (Variables|Attributes|Thirst|GetDepleteThirstByTime) (Variables|Attributes|Thirst|GetThirstDepletionRate) true))

(fn SetHealthTimer
  (Utilities|Time|SetTimerbyFunctionName self (Variables|Attributes|Health|GetDepleteHealthByTime) (Variables|Attributes|Health|GetHealthDepletionRate) true))

(fn SetHungerTimer
  (Utilities|Time|SetTimerbyFunctionName self (Variables|Attributes|Hunger|GetDepleteHungerByTime) (Variables|Attributes|Hunger|GetHungerDepletionRate) true))

(fn CanSprint?
  (return (Math|Boolean|ANDBoolean (> (Math|Vector|VectorLength (Transformation|GetVelocity)) 1e+01) (not (Variables|Attributes|Movement|GetOutOfBreath?)) (not (AI|Components|NavMovement|IsFalling (Variables|Character|GetCharacterMovement))))))

(fn SetSpeedtoSprint
  (Variables|/Script/Engine.CharacterMovementComponent|SetMaxWalkSpeed (Variables|Character|GetCharacterMovement) (Variables|Attributes|Movement|GetSprintSpeed)))

(fn SetSpeedtoWalk
  (Variables|/Script/Engine.CharacterMovementComponent|SetMaxWalkSpeed (Variables|Character|GetCharacterMovement) (Variables|Attributes|Movement|GetWalkSpeed)))

(fn SetStaminaDecreaseTimer
  (Utilities|Time|SetTimerbyFunctionName self (Variables|Attributes|Stamina|GetStaminaDecreaseByTime) (Variables|Attributes|Stamina|GetStaminaUpdateRate) true))

(fn SetStaminaIncreaseTimer
  (Utilities|Time|SetTimerbyFunctionName self (Variables|Attributes|Stamina|GetStaminaIncreaseByTime) (Variables|Attributes|Stamina|GetStaminaUpdateRate) true))

(fn ClearStaminaDecreaseTimer
  (Utilities|Time|ClearTimerbyFunctionName self (Variables|Attributes|Stamina|GetStaminaDecreaseByTime)))

(fn ClearStaminaIncreaseTimer
  (Utilities|Time|ClearTimerbyFunctionName self (Variables|Attributes|Stamina|GetStaminaIncreaseByTime)))

(fn IsPerformingAction?
  (return (Math|Boolean|ORBoolean (AI|Components|NavMovement|IsFalling (Variables|Character|GetCharacterMovement)) (Variables|Actions|GetIsGathering?) (Variables|Actions|GetIsAtacking?) (Variables|Actions|GetIsInMenu?))))

(fn SetSpeedtoCrouch
  (Variables|/Script/Engine.CharacterMovementComponent|SetMaxWalkSpeed (Variables|Character|GetCharacterMovement) (Variables|Attributes|Movement|GetCrouchSpeed)))

(fn SetWeatherManager
  (Utilities|IsValid (Variables|References|GetWeatherManagerRef)
    (:Is%20Valid
      _)
    (:Is%20Not%20Valid
      (bind _outactors (Actor|GetAllActorsOfClass "/Game/Blueprints/Weather/WeatherManager.WeatherManager_C"))))
  (Variables|References|SetWeatherManagerRef (Utilities|Array|Get(acopy) _outactors)))

(fn SetBodyTempTimer
  (Utilities|Time|SetTimerbyFunctionName self (Variables|Attributes|Temperaure|GetUpdateBodyTempFunc) (Variables|Attributes|Temperaure|GetUpdateTempRate) true))

(fn UpdateBodyTemp
  (Attributes|Temperature|ModifyBodyTemperature self (Math|Curves|GetFloatValue (Variables|Attributes|Temperaure|GetBodyTempCurveMod) (- (Attributes|Temperature|GetFeelTemp) (Variables|Attributes|Temperaure|GetDesiredBodyTemperature)))))

(fn GetFeelTemp
  (return (select (Variables|Attributes|Temperaure|GetIsWorldTempOverriten) (+ (Variables|Attributes|Temperaure|GetClothingTemperatureModifier) (Variables|Attributes|Temperaure|GetOverridenWorldTemp)) (+ (Variables|/Game/Blueprints/Weather/WeatherManager.WeatherManager_C|GetFinalWorldTemperature (Variables|References|GetWeatherManagerRef)) (Variables|Attributes|Temperaure|GetClothingTemperatureModifier) (Variables|Attributes|Temperaure|GetAreaTemperatureModifier)))))

(fn ModifyBodyTemperature
  (params (TempMultiplier :type Float%20%28single-precision%29))
  (bind _output_get (Variables|Attributes|Temperaure|SetCurrentBodyTemperature (+ (* TempMultiplier (Variables|Attributes|Temperaure|GetSpecificHeat)) (Variables|Attributes|Temperaure|GetCurrentBodyTemperature))))
  (return _output_get))

(fn ApplyTemperatureModifier
  (params (OverrideWorldTemp :type Boolean) (OverritenTemp :type Float%20%28single-precision%29) (AditionalModTemp :type Float%20%28single-precision%29))
  (Variables|Attributes|Temperaure|SetIsWorldTempOverriten OverrideWorldTemp)
  (Variables|Attributes|Temperaure|SetOverridenWorldTemp OverritenTemp)
  (Variables|Attributes|Temperaure|SetAreaTemperatureModifier (+ AditionalModTemp (Variables|Attributes|Temperaure|GetAreaTemperatureModifier))))

(fn SetIceLayoutRef
  (Utilities|IsValid (Variables|References|UI|GetIceLayoutRef)
    (:Is%20Valid
      _)
    (:Is%20Not%20Valid
      (bind _returnvalue (UserInterface|CreateWidget "/Game/UI/UI_ICEPanelLayout.UI_ICEPanelLayout_C" (Game|GetPlayerController 0) self))))
  (bind _output_get (Variables|References|UI|SetIceLayoutRef _returnvalue))
  (UserInterface|Viewport|AddtoViewport _output_get 0)
  (Widget|SetVisibility _output_get "Hidden"))

(fn UseItem
  (params (ItemToUse :type BP%20Inventory%20Item%20Object%20Reference))
  (bind _self self)
  (bind _output_get (LocalVariables|SetL_Item ItemToUse))
  (switch Utilities|FlowControl|Switch|SwitchonEItemType (Default|GetItemType (Variables|Default|GetBP_Inventory) _output_get)
    (:NewEnumerator0
      (Default|ConsumeItem (Variables|Default|GetBP_Inventory) (LocalVariables|GetL_Item))
      (bind _asbp_inventory_item_consumable (Utilities|Casting|CastToBP_InventoryItem_Consumable (LocalVariables|GetL_Item)))
      (Default|OnConsume _asbp_inventory_item_consumable _self))
    (:NewEnumerator9
      (bind _itemequiped (Default|EquipItem (Variables|Default|GetBP_Equipment) (LocalVariables|GetL_Item) :!label _label))
      (bind _asbp_inventory_item_equipable (Utilities|Casting|CastToBP_InventoryItem_Equipable (LocalVariables|GetL_Item)))
      (Default|OnEquip _asbp_inventory_item_equipable _self)
      (Default|RemoveItem (Variables|Default|GetBP_Inventory) _itemequiped))
    (:NewEnumerator11
      (goto _label))
    (:NewEnumerator12
      (goto _label))
    (:NewEnumerator13
      (goto _label))
    (:NewEnumerator14
      (goto _label))))

(fn GiveStr
  (params (Str :type Integer))
  (Variables|Attributes|SetStats (Utilities|Struct|MakeS_Stats (+ Str (.strenght (Variables|Attributes|GetStats))) (.inteligence (Variables|Attributes|GetStats)) (.dextery (Variables|Attributes|GetStats)) (.constitution (Variables|Attributes|GetStats)) (.charisma (Variables|Attributes|GetStats)))))

(fn RemoveStr
  (params (Str :type Integer)))

(fn GiveInt
  (params (Int :type Integer)))

(fn RemoveInt
  (params (Int :type Integer)))

(fn GiveChr
  (params (Chr :type Integer)))

(fn RemoveChr
  (params (Chr :type Integer)))

(fn GiveDex
  (params (Dex :type Integer)))

(fn RemoveDex
  (params (Dex :type Integer)))

(fn GiveConst
  (params (Const :type Integer)))

(fn RemoveConst
  (params (Const :type Integer)))

(fn GetStr
  (return (.strenght (Variables|Attributes|GetStats))))

(fn GetInt
  (return (.inteligence (Variables|Attributes|GetStats))))

(fn GetChr
  (return (.charisma (Variables|Attributes|GetStats))))

(fn GetDex
  (return (.dextery (Variables|Attributes|GetStats))))

(fn GetConst
  (return (.constitution (Variables|Attributes|GetStats))))

(fn TakeDamage
  (params (Damage :type Float%20%28single-precision%29))
  (bind _output_get (Variables|Attributes|Health|SetCurrentHealth (Math|Float|Clamp(Float) (- (Variables|Attributes|Health|GetCurrentHealth) Damage) 0.0 (Variables|Attributes|Health|GetMaxHealth))))
  (if (<= _output_get 0.0)
    (Development|PrintString "YourDEad")))

(fn SetSkillsWidgetRef
  (Utilities|IsValid (Variables|References|UI|GetSkillsTraitsWidgetRef)
    (:Is%20Valid
      _)
    (:Is%20Not%20Valid
      (bind _returnvalue (UserInterface|CreateWidget "/Game/UI/UI_SkillsAndTraits.UI_SkillsAndTraits_C" (Game|GetPlayerController 0)))
      (bind _output_get (Variables|References|UI|SetSkillsTraitsWidgetRef _returnvalue))))
  (UserInterface|Viewport|AddtoViewport _output_get 0))