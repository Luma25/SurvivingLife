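; BP_Bush is a berry bush actor that drops berry world items and has a limited life.
; On BeginPlay it rolls a random berry count.
; Each DoOnce event decrements Life and spawns a small berry pickup at the bush's transform.
; When Life reaches 1, the count is first halved, rounding up, and the bush remains; at any other value it drops the current count and destroys itself.
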(event EventBeginPlay
  (CallFunction|Initialize))

(event EventDoOnce
  (params (LifePoints :type Integer) (CharacterRef :type BP%20Surviving%20Life%20Character%20Object%20Reference))
  (CallFunction|RemoveLife)
  (CallFunction|Die))

(fn ConstructionScript)

(fn Initialize
  (Variables|Default|SetBerriesAmount (Math|Random|RandomIntegerinRange 1 6)))

(fn Die
  (bind _returnvalue (Transformation|GetActorTransform))
  (bind _returnvalue_2 (Transformation|GetActorTransform))
  (if (== (Variables|Default|GetLife) 1)
    (bind _output_get (Variables|Default|SetBerriesAmount (+ (Math|Integer|%(Integer) (Variables|Default|GetBerriesAmount) 2) (/ (Variables|Default|GetBerriesAmount) 2))))
    (Game|SpawnActorfromClass "/Game/Blueprints/Inventory/Actors/BP_WorldItem_Berries.BP_WorldItem_Berries_C" (Math|Transform|MakeTransform (.location _returnvalue) (.rotation _returnvalue) "0.100000,0.100000,0.100000") "AdjustIfPossibleButAlwaysSpawn" 0 _output_get 0)
    (else
      (Game|SpawnActorfromClass "/Game/Blueprints/Inventory/Actors/BP_WorldItem_Berries.BP_WorldItem_Berries_C" (Math|Transform|MakeTransform (.location _returnvalue_2) (.rotation _returnvalue_2) "0.100000,0.100000,0.100000") "AdjustIfPossibleButAlwaysSpawn" 0 (Variables|Default|GetBerriesAmount) 0)
      (Actor|DestroyActor))))

(fn RemoveLife
  (Math|Integer|DecrementInt (Variables|Default|GetLife)))