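; BP_Tree is a tree actor with a wood amount and a life value, both randomized on BeginPlay through InitializeTree.
; RemoveLife subtracts the given points from Life but does not check for death or call Die.
; Die only looks up the Material row in the DTItems data table, without using the result or destroying the actor.
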(event EventBeginPlay
  (CallFunction|InitializeTree))

(event EventDoOnce)

(fn ConstructionScript)

(fn InitializeTree
  (bind _returnvalue (Math|Random|RandomIntegerinRange 2 6))
  (Variables|Default|SetWoodAmount _returnvalue)
  (Variables|Default|SetLife _returnvalue))

(fn Die
  (Utilities|GetDataTableRow "/Game/Blueprints/Structure/DataTables/DTItems.DTItems" (Variables|Default|GetMaterial)))

(fn RemoveLife
  (params (LifePoints :type Integer))
  (Variables|Default|SetLife (- (Variables|Default|GetLife) LifePoints)))