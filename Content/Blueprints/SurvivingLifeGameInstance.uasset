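; Game instance for Surviving Life that manages LAN multiplayer sessions through host, search, join and destroy events.
; Each event runs an async session node on the first player controller and mostly reports outcomes with debug prints.
; Hosting opens GeneralMap as a listen server.
; Searching stores its results in SessionResults, and joining takes the first entry without checking that one exists.
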(event Custom|HOSTGame
  (bind _returnvalue (Game|GetPlayerController 0))
  ;[1 1 1] Host Game
  (|Session _returnvalue 5 true
    (:OnSuccess
      (Development|ExecuteConsoleCommand "open GeneralMap?listen" _returnvalue)
      (Development|PrintString "SESSION CREATED SUCCESFULLY"))
    (:OnFailure
      (Development|PrintString "SESSION COULD NOT BE CREATED"))))

(event Custom|DESTROYGame
  ;[1 1 1] Destroy Game
  (|DestroySession (Game|GetPlayerController 0)
    (:OnSuccess
      (Development|PrintString "SESSION DESTROYED SUCCESFULLY"))
    (:OnFailure
      (Development|PrintString "COULD NOT DESTROY SESSION"))))

(event Custom|JOINGame
  ;[1 1 1] Join Game
  (|JoinSession (Game|GetPlayerController 0) (Utilities|Array|Get(acopy) (Variables|Default|GetSessionResults))
    (:OnSuccess
      (Development|PrintString "JOINED SESSION SUCCESFULLY"))
    (:OnFailure
      (Development|PrintString "COULD NOT JOIN SESSION"))))

(event Custom|SEARCHGame
  ;[1 1 1] Search Game
  (bind _results (|FindSessions (Game|GetPlayerController 0) 3 true)
    (:OnSuccess
      (Variables|Default|SetSessionResults _results))
    (:OnFailure
      (Development|PrintString "SESSIONS NOT FOUND"))))