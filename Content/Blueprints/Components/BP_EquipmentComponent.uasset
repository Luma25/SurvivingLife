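; Equipment component that tracks a character's six gear slots: head, armor, legs, left hand, right hand and accessory.
; On BeginPlay it fills every slot with an empty placeholder item.
; EquipItem picks the slot from the item's type, unequips and returns any occupant, then stores the new item.
; UnEquipItem removes an equipable item's bonus from the character and restores a placeholder; bonuses are not applied in this component.
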(event EventBeginPlay
  (CallFunction|InitializeEquipment))

(event EventTick
  (params (DeltaSeconds :type Float%20%28single-precision%29)))

(fn InitializeEquipment
  (Utilities|Array|Clear (Variables|Default|GetEquipment))
  (for _index (range 0 5)
    (bind _returnvalue (Game|ConstructObjectfromClass "/Game/Blueprints/Inventory/Items/BP_InventoryItem_Empty.BP_InventoryItem_Empty_C" self))
    (Utilities|Array|Add (Variables|Default|GetEquipment) _returnvalue)))

(fn GetEquipment
  (return (Variables|Default|GetEquipment)))

(fn EquipItem
  (params (ItemToEquip :type BP%20Inventory%20Item%20Object%20Reference) (CharacterRef :type BP%20Surviving%20Life%20Character%20Object%20Reference))
  (bind _equipment (Variables|Default|GetEquipment))
  (bind _equipment_2 (Variables|Default|GetEquipment))
  (bind _equipment_3 (Variables|Default|GetEquipment))
  (bind _equipment_4 (Variables|Default|GetEquipment))
  (bind _equipment_5 (Variables|Default|GetEquipment))
  (bind _equipment_6 (Variables|Default|GetEquipment))
  (bind _output (Utilities|Array|Get(acopy) _equipment_3))
  (bind _output_2 (Utilities|Array|Get(acopy) _equipment_4 5))
  (bind _output_3 (Utilities|Array|Get(acopy) _equipment_5 1))
  (bind _output_4 (Utilities|Array|Get(acopy) _equipment_6 2))
  (bind _output_5 (Utilities|Array|Get(acopy) _equipment 3))
  (bind _output_6 (Utilities|Array|Get(acopy) _equipment_2 4))
  (bind _output_get (LocalVariables|SetL_ItemToEquip ItemToEquip))
  (switch Utilities|FlowControl|Switch|SwitchonEItemType (.type (Default|GetItemInfo _output_get))
    (:NewEnumerator9
      (if (!= _output "/Game/Blueprints/Inventory/Items/BP_InventoryItem_Empty.BP_InventoryItem_Empty")
        (bind _unequipitem (CallFunction|UnEquipItem _output CharacterRef)))
      (Utilities|Array|SetArrayElem (Variables|Default|GetEquipment) 0 (LocalVariables|GetL_ItemToEquip))
      (return _unequipitem))
    (:NewEnumerator11
      (if (!= _output_3 "/Game/Blueprints/Inventory/Items/BP_InventoryItem_Empty.BP_InventoryItem_Empty")
        (bind _unequipitem_2 (CallFunction|UnEquipItem _output_3 CharacterRef)))
      (Utilities|Array|SetArrayElem (Variables|Default|GetEquipment) 1 (LocalVariables|GetL_ItemToEquip))
      (return _unequipitem_2))
    (:NewEnumerator12
      (if (!= _output_4 "/Game/Blueprints/Inventory/Items/BP_InventoryItem_Empty.BP_InventoryItem_Empty")
        (bind _unequipitem_3 (CallFunction|UnEquipItem _output_4 CharacterRef)))
      (Utilities|Array|SetArrayElem (Variables|Default|GetEquipment) 2 (LocalVariables|GetL_ItemToEquip))
      (return _unequipitem_3))
    (:NewEnumerator13
      (if (!= _output_5 "/Game/Blueprints/Inventory/Items/BP_InventoryItem_Empty.BP_InventoryItem_Empty")
        (bind _unequipitem_4 (CallFunction|UnEquipItem _output_5 CharacterRef)))
      (Utilities|Array|SetArrayElem (Variables|Default|GetEquipment) 3 (LocalVariables|GetL_ItemToEquip))
      (return _unequipitem_4))
    (:NewEnumerator16
      (if (!= _output_6 "/Game/Blueprints/Inventory/Items/BP_InventoryItem_Empty.BP_InventoryItem_Empty")
        (bind _unequipitem_5 (CallFunction|UnEquipItem _output_6 CharacterRef)))
      (Utilities|Array|SetArrayElem (Variables|Default|GetEquipment) 4 (LocalVariables|GetL_ItemToEquip))
      (return _unequipitem_5))
    (:NewEnumerator14
      (if (!= _output_2 "/Game/Blueprints/Inventory/Items/BP_InventoryItem_Empty.BP_InventoryItem_Empty")
        (bind _unequipitem_6 (CallFunction|UnEquipItem _output_2 CharacterRef)))
      (Utilities|Array|SetArrayElem (Variables|Default|GetEquipment) 5 (LocalVariables|GetL_ItemToEquip))
      (return _unequipitem_6))))

(fn UnEquipItem
  (params (ItemToUnEquip :type BP%20Inventory%20Item%20Object%20Reference) (CharacterRef :type BP%20Surviving%20Life%20Character%20Object%20Reference))
  (bind _equipment (Variables|Default|GetEquipment))
  (bind _asbp_inventory_item_equipable (Utilities|Casting|CastToBP_InventoryItem_Equipable ItemToUnEquip))
  (Default|RemoveBonus _asbp_inventory_item_equipable CharacterRef)
  (bind _returnvalue (Game|ConstructObjectfromClass "/Game/Blueprints/Inventory/Items/BP_InventoryItem_Empty.BP_InventoryItem_Empty_C" self))
  (Utilities|Array|SetArrayElem _equipment (Utilities|Array|FindItem _equipment ItemToUnEquip) _returnvalue)
  (return ItemToUnEquip))