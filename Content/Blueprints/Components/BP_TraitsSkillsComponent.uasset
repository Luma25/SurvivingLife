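; Character component that tracks activity milestones and rewards them with named skills and stat bonuses.
; BoxerUp counts punches and grants Strength on hitting its limit, while LumberJack counts felled trees and grants Constitution on every call past its limit.
; GiveBonus routes each reward to the passed character's stat setter by stat type.
; Skill and trait lists clear on BeginPlay and have getters, but AddTrait and SetWidgetRef are empty stubs.
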(event EventBeginPlay
  (Utilities|Array|Clear (Variables|Default|GetSkills))
  (Utilities|Array|Clear (Variables|Default|GetTraits)))

(event EventTick
  (params (DeltaSeconds :type Float%20%28single-precision%29)))

(fn GiveBonus
  (params (CharacterRef :type BP%20Surviving%20Life%20Character%20Object%20Reference) (Bonus :type Integer) (StatType :type EStatType%20Enum :default "NewEnumerator0"))
  (switch Utilities|FlowControl|Switch|SwitchonEStatType StatType
    (:NewEnumerator0
      (Default|GiveStr CharacterRef Bonus))
    (:NewEnumerator1
      (Default|GiveInt CharacterRef Bonus))
    (:NewEnumerator2
      (Default|GiveDex CharacterRef Bonus))
    (:NewEnumerator3
      (Default|GiveConst CharacterRef Bonus))
    (:NewEnumerator4
      (Default|GiveChr CharacterRef Bonus))))

(fn BoxerUp
  (params (CharacterRef :type BP%20Surviving%20Life%20Character%20Object%20Reference))
  (bind _result (Math|Integer|IncrementInt (Variables|BoxerSkill|GetPunchAmount))
    (:%20%20
      (if (== _result (Variables|BoxerSkill|GetMaxPunch))
        (CallFunction|GiveBonus CharacterRef (Variables|BoxerSkill|GetPunchBonus) "NewEnumerator0")
        (CallFunction|AddSkill "Boxer Up")))))

(fn LumberJack
  (params (CharacterRef :type BP%20Surviving%20Life%20Character%20Object%20Reference))
  (bind _result (Math|Integer|IncrementInt (Variables|LumberJackSkill|GetTreesDead))
    (:%20%20
      (if (> _result (Variables|LumberJackSkill|GetMaxTrees))
        (CallFunction|GiveBonus CharacterRef (Variables|LumberJackSkill|GetTreesBonus) "NewEnumerator3")
        (CallFunction|AddSkill "LumberJack")))))

(fn SetWidgetRef)

(fn GetSkills
  (return (Variables|Default|GetSkills)))

(fn GetTraits
  (return (Variables|Default|GetTraits)))

(fn AddSkill
  (params (Skill%20Name :type Name))
  (Utilities|Array|Add (Variables|Default|GetSkills) Skill%20Name))

(fn AddTrait)