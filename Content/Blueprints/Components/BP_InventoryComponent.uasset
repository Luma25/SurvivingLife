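; Inventory component that holds items as objects in a fixed number of slots, using BP_InventoryItem_Empty instances as placeholders for free slots.
; AddItem requires a free slot, tops up matching stackable items and puts overflow into the first empty one.
; ConsumeItem decrements or removes items, RemoveItem blanks a slot, and GetItemOfEach tallies amounts per class as SIngredientes structs.
; EquipItem is an empty stub.
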(event EventBeginPlay
  (CallFunction|InitializeInventory))

(fn GetInventory
  (return (Variables|Default|GetInventory)))

(fn InitializeInventory
  (Utilities|Array|Clear (Variables|Default|GetInventory))
  (for _index (range 0 (- (Variables|Default|GetSlots) 1))
    (bind _returnvalue (Game|ConstructObjectfromClass "/Game/Blueprints/Inventory/Items/BP_InventoryItem_Empty.BP_InventoryItem_Empty_C" self))
    (Utilities|Array|Add (Variables|Default|GetInventory) _returnvalue)))

(fn AddItem
  (params (ItemToAdd :type BP%20Inventory%20Item%20Class%20Reference) (AmountToAdd :type Integer))
  (bind (_hasspaces _open_spaces) (CallFunction|HasSpaceinInventory))
  (LocalVariables|SetL_ItemClass ItemToAdd)
  (LocalVariables|SetL_Amount AmountToAdd)
  (if _hasspaces
    (LocalVariables|SetL_OpenSpaces _open_spaces)
    (for _array_element (Variables|Default|GetInventory)
      (if (== (Utilities|GetClass _array_element) (LocalVariables|GetL_ItemClass))
        (bind _output_get (LocalVariables|SetL_Item _array_element))
        (if (Default|CanStack? _output_get)
          (if (> (Default|GetRoomonStack (LocalVariables|GetL_Item)) 0)
            (if (<= (+ (Default|GetAmount (LocalVariables|GetL_Item)) (LocalVariables|GetL_Amount)) (Default|GetMaxStackAmount (LocalVariables|GetL_Item)))
              (Default|SetAmount (LocalVariables|GetL_Item) (+ (Default|GetAmount (LocalVariables|GetL_Item)) (LocalVariables|GetL_Amount)))
              (return true)
              (elif (> (LocalVariables|GetL_OpenSpaces) 0)
                (LocalVariables|SetL_Amount (- (LocalVariables|GetL_Amount) (Default|GetRoomonStack (LocalVariables|GetL_Item))))
                (Default|SetAmount (LocalVariables|GetL_Item) (Default|GetMaxStackAmount (LocalVariables|GetL_Item)))
                (bind (_array_element_2 _array_index) (Utilities|Array|ForEachLoopwithBreak (Variables|Default|GetInventory) :!label _label)
                  (:LoopBody
                    (if (== (Utilities|GetClass _array_element_2) "/Game/Blueprints/Inventory/Items/BP_InventoryItem_Empty.BP_InventoryItem_Empty_C")
                      (LocalVariables|SetL_Index _array_index)
                      (goto _label Break)
                      (else
                        (LocalVariables|SetL_Index -1))))
                  (:Completed
                    (if (>= (LocalVariables|GetL_Index) 0)
                      (bind _returnvalue (Game|ConstructObjectfromClass (LocalVariables|GetL_ItemClass) self))
                      (Default|SetAmount _returnvalue (LocalVariables|GetL_Amount))
                      (Utilities|Array|SetArrayElem (Variables|Default|GetInventory) (LocalVariables|GetL_Index) _returnvalue)
                      (return true)
                      (else
                        (return false)))))
                (else
                  (return false)))))
          (else
            (goto _label)))))
    (bind (_array_element_3 _array_index_2) (Utilities|Array|ForEachLoopwithBreak (Variables|Default|GetInventory) :!label _label_2)
      (:LoopBody
        (if (== (Utilities|GetClass _array_element_3) "/Game/Blueprints/Inventory/Items/BP_InventoryItem_Empty.BP_InventoryItem_Empty_C")
          (LocalVariables|SetL_Index _array_index_2)
          (goto _label_2 Break)
          (else
            (LocalVariables|SetL_Index -1))))
      (:Completed
        (if (>= (LocalVariables|GetL_Index) 0)
          (bind _returnvalue_2 (Game|ConstructObjectfromClass (LocalVariables|GetL_ItemClass) self))
          (Default|SetAmount _returnvalue_2 (LocalVariables|GetL_Amount))
          (Utilities|Array|SetArrayElem (Variables|Default|GetInventory) (LocalVariables|GetL_Index) _returnvalue_2)
          (return true)
          (else
            (return false)))))
    (else
      (return false))))

(fn HasSpaceinInventory
  (bind _l_openspaces (LocalVariables|GetL_OpenSpaces))
  (for _array_element (Variables|Default|GetInventory)
    (if (== (Utilities|GetClass _array_element) "/Game/Blueprints/Inventory/Items/BP_InventoryItem_Empty.BP_InventoryItem_Empty_C")
      (Math|Integer|IncrementInt (LocalVariables|GetL_OpenSpaces))))
  (return (> _l_openspaces 0) _l_openspaces))

(fn GetItemType
  (params (Item :type BP%20Inventory%20Item%20Object%20Reference))
  (return (.type (Default|GetItemInfo Item))))

(fn ConsumeItem
  (params (ItemToConsume :type BP%20Inventory%20Item%20Object%20Reference))
  (bind _inventory (Variables|Default|GetInventory))
  (bind _inventory_2 (Variables|Default|GetInventory))
  (bind _output_get (LocalVariables|SetL_Item (Utilities|Array|Get(acopy) _inventory (Utilities|Array|FindItem _inventory ItemToConsume))))
  (if (== (Default|GetAmount _output_get) 1)
    (bind _returnvalue (Utilities|Array|RemoveItem _inventory_2 (LocalVariables|GetL_Item)))
    (if _returnvalue
      (bind _returnvalue_2 (Game|ConstructObjectfromClass "/Game/Blueprints/Inventory/Items/BP_InventoryItem_Empty.BP_InventoryItem_Empty_C" self))
      (Utilities|Array|Add _inventory_2 _returnvalue_2))
    (else
      (Default|SetAmount (LocalVariables|GetL_Item) (- (Default|GetAmount _output_get) 1)))))

(fn EquipItem)

(fn RemoveItem
  (params (ItemToRemove :type BP%20Inventory%20Item%20Object%20Reference))
  (bind _returnvalue (Game|ConstructObjectfromClass "/Game/Blueprints/Inventory/Items/BP_InventoryItem_Empty.BP_InventoryItem_Empty_C" self))
  (Utilities|Array|SetArrayElem (Variables|Default|GetInventory) (Utilities|Array|FindItem (Variables|Default|GetInventory) ItemToRemove) _returnvalue))

(fn GetItemOfEach
  (for _array_element (Variables|Default|GetInventory)
    (bind _output_get (LocalVariables|SetL_Item _array_element))
    (bind _array_element_2 (Utilities|Array|ForEachLoopwithBreak (LocalVariables|GetItemOfEach) :!label _label)
      (:LoopBody
        (if (== (.item _array_element_2) (Utilities|GetClass _output_get))
          (Utilities|Array|SetArrayElem (LocalVariables|GetItemOfEach) 0 (Utilities|Struct|MakeS_Ingredientes (.item _array_element_2) (+ (Default|GetAmount (LocalVariables|GetL_Item)) (.amount _array_element_2))))
          (goto _label Break)))
      (:Completed
        (Utilities|Array|Add (LocalVariables|GetItemOfEach) (Utilities|Struct|MakeS_Ingredientes (Utilities|GetClass _output_get) (Default|GetAmount _output_get))))))
  (return (LocalVariables|GetItemOfEach)))